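; Tank_BP is a player-controlled tank that drives by applying physics forces to its TankBody.
; MoveForward pushes behind the body's origin and MoveRight pushes sideways ahead of it to steer, with both forces scaled by delta time and cut off above a speed limit.
; The forward axis also runs PreventDrifting, which counters sideways slip found by a velocity dot product.
; Look axes feed controller pitch and yaw, and Tick prints speed.
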(event EventTick
  (params (DeltaSeconds :type Float%20%28single-precision%29))
  (Development|PrintString (Utilities|String|ToString(Float) (Math|Vector|VectorLength (Transformation|GetVelocity)))))

(event Input|AxisEvents|InputAxisMoveForward
  (params (AxisValue :type Float%20%28single-precision%29))
  (Class|PrimitiveComponent|AddForceatLocation (Variables|Default|GetTank_Body) (CallFunction|GetForcetoApply AxisValue (Math|Vector|GetForwardVector (Variables|Default|GetTank_Body)) (Variables|Default|GetForwardForcePerSec) (Variables|Default|GetMaxForwardVelocity)) (CallFunction|GetForceApplyLocation -2e+02) "None")
  (CallFunction|PreventDrifting))

(event Input|AxisEvents|InputAxisMoveRight
  (params (AxisValue :type Float%20%28single-precision%29))
  (Class|PrimitiveComponent|AddForceatLocation (Variables|Default|GetTank_Body) (CallFunction|GetForcetoApply AxisValue (Math|Vector|GetRightVector (Variables|Default|GetTank_Body)) (Variables|Default|GetTurningForcePerSec) 1e+04) (CallFunction|GetForceApplyLocation 3e+02) "None"))

(event Input|AxisEvents|InputAxisLookUp
  (params (AxisValue :type Float%20%28single-precision%29))
  (Pawn|Input|AddControllerPitchInput AxisValue))

(event Input|AxisEvents|InputAxisLookRight
  (params (AxisValue :type Float%20%28single-precision%29))
  (Pawn|Input|AddControllerYawInput AxisValue))

(fn ConstructionScript)

(fn GetForceApplyLocation
  (params (Offset :type Float%20%28single-precision%29))
  (bind _tank_body (Variables|Default|GetTank_Body))
  (return (+ (Transformation|GetWorldLocation _tank_body) (* (Math|Vector|GetForwardVector _tank_body) Offset))))

(fn GetForcetoApply
  (params (AxisValue :type Float%20%28single-precision%29) (Direction :type Vector) (ForcePerSec :type Float%20%28single-precision%29) (MaxVelocity :type Float%20%28single-precision%29))
  (if (< (Math|Vector|VectorLength (Transformation|GetVelocity)) MaxVelocity)
    (return (* Direction (* AxisValue ForcePerSec (Utilities|Time|GetWorldDeltaSeconds))))
    (else
      (return "0, 0, 0"))))

(fn PreventDrifting
  (Physics|AddForce (Variables|Default|GetTank_Body) (* (Transformation|GetActorRightVector) (* (Math|Vector|DotProduct (Transformation|GetVelocity) (Transformation|GetActorRightVector)) (Utilities|Time|GetWorldDeltaSeconds) -1.0 (Physics|GetMass (Variables|Default|GetTank_Body)) 1.0)) "None" true))