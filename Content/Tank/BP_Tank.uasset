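; Physics-driven tank pawn with player input for driving, looking, camera switching and firing.
; Driving applies offset forces to TankBody under speed limits, with a counter-force against sideways drift when driving forward or back.
; Helpers, not called here, turn turret and barrel at limited rates toward the crosshair or player pawn, using ballistic prediction for the latter.
; Firing spawns a projectile and particles at every barrel socket; damage reduces and prints Health.
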(event Game|Damage|EventAnyDamage
  (params (Damage :type Float%20%28single-precision%29) (DamageType :type Damage%20Type%20Object%20Reference) (InstigatedBy :type Controller%20Object%20Reference) (DamageCauser :type Actor%20Object%20Reference))
  (bind _output_get (Variables|General|SetHealth (- (Variables|General|GetHealth) Damage)))
  (Development|PrintString (Utilities|String|ToString(Float) _output_get)))

(event Input|ActionEvents|InputActionSwitchCamera
  (params (Key :type Key%20Structure))
  ;[1 1 1] Camera Switch
  (:Pressed
    (Components|Activation|ToggleActive (Variables|Default|GetThirdPerson))
    (Components|Activation|ToggleActive (Variables|Default|GetFirstPerson))))

(event Input|ActionEvents|InputActionFire
  (params (Key :type Key%20Structure))
  (:Pressed
    (CallFunction|SpawnProjectile)))

(event Input|AxisEvents|InputAxisMoveForward
  (params (AxisValue :type Float%20%28single-precision%29))
  ;[1 1 1] Pawn Movement
  (bind _return_value (CallFunction|CheckMaxLinearVelocity (Variables|Speed|GetMaxLinearVelocity)))
  (if _return_value
    (Class|PrimitiveComponent|AddForceatLocation (Variables|Default|GetTankBody) (CallFunction|GetForcetoApply AxisValue (Math|Vector|GetForwardVector (Variables|Default|GetTankBody)) (Variables|Speed|GetForwardForce)) (CallFunction|GetForceApplyLocation -2e+02) "None")
    (CallFunction|PreventDrifting)))

(event Input|AxisEvents|InputAxisMoveRight
  (params (AxisValue :type Float%20%28single-precision%29))
  ;[1 1 1] Pawn Movement
  (bind _returnvalue (CallFunction|CheckMaxAngularVelocity (Variables|Speed|GetMaxAngularVelocity)))
  (if _returnvalue
    (Class|PrimitiveComponent|AddForceatLocation (Variables|Default|GetTankBody) (CallFunction|GetForcetoApply AxisValue (Math|Vector|GetRightVector (Variables|Default|GetTankBody)) (Variables|Speed|GetTurningForce)) (CallFunction|GetForceApplyLocation 3e+02) "None")))

(event Input|AxisEvents|InputAxisLookUp
  (params (AxisValue :type Float%20%28single-precision%29))
  ;[1 1 1] Mouse Movement
  (Pawn|Input|AddControllerPitchInput AxisValue))

(event Input|AxisEvents|InputAxisLookRight
  (params (AxisValue :type Float%20%28single-precision%29))
  ;[1 1 1] Mouse Movement
  (Pawn|Input|AddControllerYawInput AxisValue))

(fn ConstructionScript)

(fn GetForceApplyLocation
  (params (Offset :type Float%20%28single-precision%29))
  (bind _tankbody (Variables|Default|GetTankBody))
  (return (+ (Transformation|GetWorldLocation _tankbody) (* (Math|Vector|GetForwardVector _tankbody) Offset))))

(fn GetForcetoApply
  (params (AxisValue :type Float%20%28single-precision%29) (Direction :type Vector) (ForcePerSec :type Float%20%28single-precision%29))
  (return (* Direction (* AxisValue ForcePerSec))))

(fn PreventDrifting
  (Physics|AddForce (Variables|Default|GetTankBody) (* (Transformation|GetActorRightVector) (* (/ (Math|Vector|DotProduct (Transformation|GetVelocity) (Transformation|GetActorRightVector)) (Utilities|Time|GetWorldDeltaSeconds)) -1.0 (Physics|GetMass (Variables|Default|GetTankBody)))) "None" false))

(fn AimTurretatCrosshair
  (bind _worlddirection (CallFunction|DeprojectCrosshairtoWorld))
  (bind _tankturret (Variables|Default|GetTankTurret))
  (bind _tankturret_2 (Variables|Default|GetTankTurret))
  (bind (_x _y) (Math|Vector|BreakVector _worlddirection))
  (bind _returnvalue (Math|Vector|GetForwardVector _tankturret))
  (bind _relativerotation (Variables|/Script/Engine.SceneComponent|GetRelativeRotation _tankturret_2))
  (bind (_x_2 _y_2) (Math|Vector|BreakVector _returnvalue))
  (bind (_roll _pitch) (Math|Rotator|BreakRotator _relativerotation))
  (if (not (Math|Vector|Equal(Vector) (Math|Vector|MakeVector _x _y 0.0) (Math|Vector|MakeVector _x_2 _y_2 0.0) 0.001))
    (Transformation|SetRelativeRotation (Variables|Default|GetTankTurret) (Math|Rotator|MakeRotator _roll _pitch (CallFunction|CalculateRotationAmount _worlddirection _returnvalue (Variables|Speed|GetMaxTurretTurnSpeedDegrees) 2 (Variables|/Script/Engine.SceneComponent|GetRelativeRotation (Variables|Default|GetTankTurret)))) false false)))

(fn DeprojectCrosshairtoWorld
  (bind _returnvalue (Viewport|GetViewportSize))
  (bind _returnvalue_2 (Game|GetPlayerController 0))
  (bind (_x _y) (Math|Vector2D|BreakVector2D _returnvalue))
  (bind _returnvalue_3 (/ _x 2.0))
  (bind _returnvalue_4 (/ _y 1e+02))
  (bind _returnvalue_5 (* _returnvalue_4 3e+01))
  (bind _returnvalue_6 (Math|Vector2D|MakeVector2D _returnvalue_3 _returnvalue_5))
  (bind (_worldposition _worlddirection _returnvalue_7) (Class|GameplayStatics|DeprojectScreentoWorld _returnvalue_2 _returnvalue_6))
  (return _worldposition _worlddirection _returnvalue_7))

(fn AimBarrelatCrosshair
  (bind _worlddirection (CallFunction|DeprojectCrosshairtoWorld))
  (bind _tankbarrel (Variables|Default|GetTankBarrel))
  (bind _returnvalue (Math|Vector|GetForwardVector _tankbarrel))
  (if (not (Math|Vector|Equal(Vector) (Math|Vector|MakeVector 0.0 0.0 (.Z (Math|Vector|BreakVector _worlddirection))) (Math|Vector|MakeVector 0.0 0.0 (.Z (Math|Vector|BreakVector _returnvalue))) 0.001))
    (Transformation|SetRelativeRotation (Variables|Default|GetTankBarrel) (Math|Rotator|MakeRotator 0.0 (Math|Float|Clamp(Float) (CallFunction|CalculateRotationAmount _worlddirection _returnvalue (Variables|Speed|GetMaxBarrelTurnSpeedDegrees) 1 (Variables|/Script/Engine.SceneComponent|GetRelativeRotation (Variables|Default|GetTankBarrel))) -1.0 6e+01) 0.0) false false)))

(fn CheckMaxAngularVelocity
  (params (Max%20Velocity :type Float%20%28single-precision%29))
  (bind _returnvalue (Physics|GetPhysicsAngularVelocityinDegrees (Variables|Default|GetTankBody) "None"))
  (return (<= (Math|Float|Absolute(Float) (.Z (Math|Vector|BreakVector _returnvalue))) Max%20Velocity)))

(fn CheckMaxLinearVelocity
  (params (Max%20Velocity :type Float%20%28single-precision%29))
  (return (< (Math|Vector|VectorLength (Transformation|GetVelocity)) Max%20Velocity)))

(fn SpawnProjectile
  (bind _tankbarrel (Variables|Default|GetTankBarrel))
  (for _array_element (Transformation|GetAllSocketNames _tankbarrel)
    (Game|SpawnActorfromClass (Variables|Combat|GetProjectileType) (Transformation|GetSocketTransform _tankbarrel _array_element "RTS_World") "Undefined" 0 (Variables|Combat|GetProjectileSpeed) 7.0 self)
    (Effects|SpawnEmitterAttached (Variables|Combat|GetParticleSystem) (Variables|Default|GetTankBarrel) "None" (- (.Location (Math|Transform|BreakTransform (Transformation|GetSocketTransform _tankbarrel _array_element "RTS_World"))) (* (Math|Vector|GetForwardVector (Variables|Default|GetTankBarrel)) 5e+01)) (.Rotation (Math|Transform|BreakTransform (Transformation|GetSocketTransform _tankbarrel _array_element "RTS_World"))) (.Scale (Math|Transform|BreakTransform (Transformation|GetSocketTransform _tankbarrel _array_element "RTS_World"))) "KeepWorldPosition")))

(fn AimTurretatPlayer
  (bind _returnvalue (Game|Player|GetPlayerPawn 0))
  (bind _returnvalue_2 (Transformation|GetActorLocation))
  (bind _tankturret (Variables|Default|GetTankTurret))
  (bind _returnvalue_3 (Math|Vector|GetForwardVector _tankturret))
  (bind _returnvalue_4 (Transformation|GetActorLocation _returnvalue))
  (bind (_x _y) (Math|Vector|BreakVector _returnvalue_3))
  (bind _returnvalue_5 (Math|Vector|GetUnitDirection(Vector) _returnvalue_2 _returnvalue_4))
  (bind (_x_2 _y_2) (Math|Vector|BreakVector _returnvalue_5))
  (if (not (Math|Vector|Equal(Vector) (Math|Vector|MakeVector _x_2 _y_2 0.0) (Math|Vector|MakeVector _x _y 0.0) 0.001))
    (Transformation|SetRelativeRotation (Variables|Default|GetTankTurret) (Math|Rotator|MakeRotator 0.0 0.0 (CallFunction|CalculateRotationAmount _returnvalue_5 _returnvalue_3 (Variables|Speed|GetMaxTurretTurnSpeedDegrees) 2 (Variables|/Script/Engine.SceneComponent|GetRelativeRotation (Variables|Default|GetTankTurret)))) false false)))

(fn AimBarrelatPlayer
  (params (Random%20Offset :type Vector))
  (bind _tankbarrel (Variables|Default|GetTankBarrel))
  (bind _returnvalue (Math|Vector|GetForwardVector _tankbarrel))
  (bind _tossvelocity (Class|GameplayStatics|BlueprintSuggestProjectileVelocity (Transformation|GetSocketLocation (Variables|Default|GetTankBarrel) "Projectile") (+ (Transformation|GetActorLocation (Game|Player|GetPlayerPawn 0)) Random%20Offset) (Variables|Combat|GetProjectileSpeed) 0.0 "DoNotTrace" 0.0 false false))
  (if (not (Math|Vector|Equal(Vector) (Math|Vector|MakeVector 0.0 0.0 (.Z (Math|Vector|BreakVector (Math|Vector|Normalize _tossvelocity)))) (Math|Vector|MakeVector 0.0 0.0 (.Z (Math|Vector|BreakVector _returnvalue))) 0.001))
    (Transformation|SetRelativeRotation (Variables|Default|GetTankBarrel) (Math|Rotator|MakeRotator 0.0 (Math|Float|Clamp(Float) (CallFunction|CalculateRotationAmount (Math|Vector|Normalize _tossvelocity) _returnvalue (Variables|Speed|GetMaxBarrelTurnSpeedDegrees) 1 (Variables|/Script/Engine.SceneComponent|GetRelativeRotation (Variables|Default|GetTankBarrel))) -1.0 6e+01) 0.0) false false)))

(fn CalculateRotationAmount
  (params (FirstDirection :type Vector) (Second%20Direction :type Vector) (Max%20Speed :type Float%20%28single-precision%29) (RollPitchYaw :type Integer) (RelativeRotation :type Rotator))
  (bind _returnvalue (Math|Conversions|RotationFromXVector FirstDirection))
  (bind _returnvalue_2 (Math|Conversions|RotationFromXVector Second%20Direction))
  (bind _returnvalue_3 (Utilities|Time|GetWorldDeltaSeconds))
  (bind (_roll _pitch _yaw) (Math|Rotator|BreakRotator RelativeRotation))
  (bind _returnvalue_4 (Math|Rotator|Delta(Rotator) _returnvalue _returnvalue_2))
  (bind (_roll_2 _pitch_2 _yaw_2) (Math|Rotator|BreakRotator _returnvalue_4))
  (bind _returnvalue_5 (Utilities|Select :Index RollPitchYaw :Option%200 _roll_2 :Option%201 _pitch_2 :Option%202 _yaw_2))
  (bind _returnvalue_6 (Math|Float|Clamp(Float) _returnvalue_5 -1.0))
  (bind _returnvalue_7 (* Max%20Speed _returnvalue_6 _returnvalue_3))
  (return (+ (select (< (Math|Float|Absolute(Float) _returnvalue_5) _returnvalue_7) _returnvalue_5 _returnvalue_7) (Utilities|Select :Index RollPitchYaw :Option%200 _roll :Option%201 _pitch :Option%202 _yaw))))