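; AI controller that makes its possessed BP_Tank aim and fire at the player.
; BeginPlay caches the tank and rolls a random XYZ aim offset from configurable min/max ranges.
; Tick tracks the player with turret and barrel every frame, applying the offset to barrel aim.
; A Delay on Tick throttles firing to roughly every two seconds, re-rolling the offset after each shot to vary accuracy.
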(event EventBeginPlay
  (bind (_randomoffsetx _randomoffsety _randomoffsetz) (CallFunction|GetRandomValuesforOffset))
  (bind _asbp_tank (Utilities|Casting|CastToBP_Tank (Pawn|GetControlledPawn)))
  (Variables|Default|SetControlledTank _asbp_tank)
  (Variables|Default|SetRandomOffset (Math|Vector|MakeVector _randomoffsetx _randomoffsety _randomoffsetz)))

(event EventTick
  (params (DeltaSeconds :type Float%20%28single-precision%29))
  (bind (_randomoffsetx _randomoffsety _randomoffsetz) (CallFunction|GetRandomValuesforOffset))
  (bind _controlledtank (Variables|Default|GetControlledTank))
  (Utilities|IsValid _controlledtank
    (:Is%20Valid
      (Default|AimTurretatPlayer _controlledtank)
      (Default|AimBarrelatPlayer _controlledtank (Variables|Default|GetRandomOffset))
      (Utilities|FlowControl|Delay 2.0)
      (Default|SpawnProjectile _controlledtank)
      (Variables|Default|SetRandomOffset (Math|Vector|MakeVector _randomoffsetx _randomoffsety _randomoffsetz)))))

(fn ConstructionScript)

(fn GetRandomValuesforOffset
  (bind _randomoffsetx (Variables|Default|GetRandomOffsetX))
  (bind _randomoffsety (Variables|Default|GetRandomOffsetY))
  (bind _randomoffsetz (Variables|Default|GetRandomOffsetZ))
  (bind (_x _y) (Math|Vector2D|BreakVector2D _randomoffsetz))
  (bind (_x_2 _y_2) (Math|Vector2D|BreakVector2D _randomoffsetx))
  (bind (_x_3 _y_3) (Math|Vector2D|BreakVector2D _randomoffsety))
  (return (Math|Random|RandomFloatinRange _x_2 _y_2) (Math|Random|RandomFloatinRange _x_3 _y_3) (Math|Random|RandomFloatinRange _x _y)))