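; BP_ProjectileMaster is a projectile, by name a base class, that deals radial damage on impact in a tank game.
; Construction applies speed, lifespan and mass, and BeginPlay attaches a separately spawned particle actor.
; The first hit pushes a struck BP_Tank by mass, fires a radial impulse and applies falloff damage.
; With DestroyOnHit, it deactivates the particles, gives their actor its own lifespan and destroys itself.
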(event EventBeginPlay
  (bind _returnvalue (Game|SpawnActorfromClass "/Game/Particles/BP_ParticleSystem.BP_ParticleSystem_C" (Transformation|GetActorTransform) "Undefined" 0 (Variables|Particle|GetParticleEffect) 1e+01 0))
  (Transformation|AttachActorToActor _returnvalue self "None" "SnapToTarget" "SnapToTarget" "SnapToTarget" true)
  (Variables|Particle|SetParticleSystem _returnvalue))

(event Collision|EventHit
  (params (MyComp :type Primitive%20Component%20Object%20Reference) (Other :type Actor%20Object%20Reference) (OtherComp :type Primitive%20Component%20Object%20Reference) (bSelfMoved :type Boolean) (HitLocation :type Vector :default "0, 0, 0") (HitNormal :type Vector :default "0, 0, 0") (NormalImpulse :type Vector :default "0, 0, 0") (Hit :type Hit%20Result%20Structure%20%28by%20ref%29))
  (bind _radialforce (Variables|Default|GetRadialForce))
  (bind _particlesystem (Variables|Particle|GetParticleSystem))
  (Utilities|FlowControl|DoOnce false
    (:Completed
      (Utilities|FlowControl|Sequence
        (:then_0
          (Utilities|Casting|CastToBP_Tank Other)
          (Class|PrimitiveComponent|AddForceatLocation OtherComp (* (* (Math|Vector|NegateVector HitNormal) (Variables|General|GetMass)) 1e+05) HitLocation "None"))
        (:then_1
          (Class|RadialForceComponent|FireImpulse _radialforce)
          (Class|GameplayStatics|ApplyRadialDamagewithFalloff (Variables|General|GetDamage) 0.0 HitLocation 0.0 (Variables|/Script/Engine.RadialForceComponent|GetRadius _radialforce) 1.0 0 (Utilities|Array|MakeArray self) 0 0 "ECC_Visibility")
          (if (Variables|General|GetDestroyOnHit?)
            (Components|Activation|Deactivate (Variables|/Game/Particles/BP_ParticleSystem.BP_ParticleSystem_C|GetParticleSystem _particlesystem))
            (Actor|SetLifeSpan _particlesystem (Variables|/Game/Particles/BP_ParticleSystem.BP_ParticleSystem_C|GetLifeSpan _particlesystem))
            (Actor|DestroyActor)))))))

(fn ConstructionScript
  (Variables|/Script/Engine.ProjectileMovementComponent|SetInitialSpeed (Variables|Default|GetProjectileMovement) (Variables|General|GetInitialSpeed))
  (Actor|SetLifeSpan (Variables|General|GetLifeSpan))
  (Class|PrimitiveComponent|SetMassOverrideinKg (Variables|Default|GetMesh) "None" (Variables|General|GetMass) true))