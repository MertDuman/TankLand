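; BP_Projectile is a projectile that deals explosive radial damage on its first hit.
; Construction applies configurable initial speed, lifespan and mass override.
; A DoOnce-gated Hit event pushes a struck BP_Tank component along the inverted hit normal, scaled by mass.
; It then fires a RadialForce impulse, applies falloff damage using that component's radius, and optionally destroys itself.
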(event Collision|EventHit
  (params (MyComp :type Primitive%20Component%20Object%20Reference) (Other :type Actor%20Object%20Reference) (OtherComp :type Primitive%20Component%20Object%20Reference) (bSelfMoved :type Boolean) (HitLocation :type Vector :default "0, 0, 0") (HitNormal :type Vector :default "0, 0, 0") (NormalImpulse :type Vector :default "0, 0, 0") (Hit :type Hit%20Result%20Structure%20%28by%20ref%29))
  (bind _radialforce (Variables|Default|GetRadialForce))
  (Utilities|FlowControl|DoOnce false
    (:Completed
      (Utilities|FlowControl|Sequence
        (:then_0
          (Utilities|Casting|CastToBP_Tank Other)
          (Class|PrimitiveComponent|AddForceatLocation OtherComp (* (* (Math|Vector|NegateVector HitNormal) (Variables|Default|GetMass)) 1e+04) HitLocation "None"))
        (:then_1
          (Class|RadialForceComponent|FireImpulse _radialforce)
          (Class|GameplayStatics|ApplyRadialDamagewithFalloff (Variables|Default|GetDamage) 0.0 HitLocation 0.0 (Variables|/Script/Engine.RadialForceComponent|GetRadius _radialforce) 1.0 0 (Utilities|Array|MakeArray self) 0 0 "ECC_Visibility")
          (if (Variables|Default|GetDestroyOnHit?)
            (Actor|DestroyActor)))))))

(fn ConstructionScript
  (Variables|/Script/Engine.ProjectileMovementComponent|SetInitialSpeed (Variables|Default|GetProjectileMovement) (Variables|Default|GetInitialSpeed))
  (Actor|SetLifeSpan (Variables|Default|GetLifeSpan))
  (Class|PrimitiveComponent|SetMassOverrideinKg (Variables|Default|GetMesh) "None" (Variables|Default|GetMass) true))